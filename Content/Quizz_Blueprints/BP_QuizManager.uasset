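; Quiz manager that runs a session from Panoramix's rules screen through questions, answer feedback and a final score, then returns to MainMenu after a delay.
; The construction script builds the question list from DT_QuestionList, using GI_Quiz for count and optional shuffle.
; Widget events drive the loop: each selection is compared to the first listed correct answer and scored, then Next advances the index until the list ends.
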(event `self.ReceiveBeginPlay`
  (bind _panoramixruleswidget (`self.PanoramixRulesWidget`))
  (`EnhancedInputSubsystemInterface.AddMappingContext` (pcsubsystem `EnhancedInputLocalPlayerSubsystem` (`GameplayStatics.GetPlayerController` 0)) "/Game/Quizz_Inputs/IMC_Quizz.IMC_Quizz" 0 (struct))
  ;[1 1 1] Generates the required widgets
  (bind _returnvalue (`|CreateWidget` "/Game/Quizz_UI/Quizz/WBP_QuestionWidget.WBP_QuestionWidget_C"))
  (set `self.QuestionWidget` _returnvalue)
  (bind _returnvalue_2 (`|CreateWidget` "/Game/Quizz_UI/Quizz/WBP_AnswerWidget.WBP_AnswerWidget_C"))
  (set `self.AnswerWidget` _returnvalue_2)
  ;[1 1 1] Panoramix explains the rules
  (bind _returnvalue_3 (`|CreateWidget` "/Game/Quizz_UI/Quizz/WBP_Panoramix_Speaking.WBP_Panoramix_Speaking_C"))
  (set `self.PanoramixRulesWidget` _returnvalue_3)
  (`UserWidget.AddToViewport` _panoramixruleswidget 0)
  (add `/Game/Quizz_UI/Quizz/WBP_Panoramix_Speaking.OnPanoramixStartPressed` _panoramixruleswidget (delegate `StartQuestions`)))

(event `StartQuestions`
  ;[1 1 1] Panoramix explains the rules
  (`Widget.RemoveFromParent` (`self.PanoramixRulesWidget`))
  (`self.AskQuestionEvent`))

(event `AskQuestionEvent`
  (bind _questionwidget (`self.QuestionWidget`))
  (`Widget.RemoveFromParent` (`self.AnswerWidget`))
  (bind _output (`self.GetCurrentQuestion`))
  (`/Game/Quizz_UI/Quizz/WBP_QuestionWidget.Display Question` _questionwidget _output) ; Set the question widget so it registers the question to display
  (add `/Game/Quizz_UI/Quizz/WBP_QuestionWidget.OnAnswerSelected` _questionwidget (delegate `CheckAnswerEvent`)) ; Asks the QuizManager to listen for which answer will be selected !
  (`UserWidget.AddToViewport` (`self.QuestionWidget`) 0))

(event `CheckAnswerEvent`
  (params (SelectedAnswer :type Text))
  (bind _isanswergood (`self.CheckAnswer` SelectedAnswer))
  (bind _output_get (set `self.CurrentQuestionCorrect` _isanswergood))
  (if _output_get
    (`/Engine/EditorBlueprintResources/StandardMacros.IncrementInt` (`self.TotalScore`)
      (:`  `
        _)))
  (`self.DisplayAnswerScreen` (`self.CurrentQuestionCorrect`)))

(event `DisplayAnswerScreen`
  (params (Answered :type Boolean))
  (bind _answerwidget (`self.AnswerWidget`))
  (`Widget.RemoveFromParent` (`self.QuestionWidget`))
  (bind _output (`self.GetCurrentQuestion`))
  (`/Game/Quizz_UI/Quizz/WBP_AnswerWidget.DisplayAnswer` _answerwidget (`.AnswerText_16_60BFE8164A18F9190D041CA773BE0F02` (break `/Game/Quizz_Blueprints/ST_QuestionData` _output)) Answered)
  (add `/Game/Quizz_UI/Quizz/WBP_AnswerWidget.OnNextPressed` _answerwidget (delegate `GoToNextQuestion`)) ; When button "suivant" is pressed, do it
)

(event `GoToNextQuestion`
  (bind _output_get (set `self.CurrentQuestionIndex` (+ (`self.CurrentQuestionIndex`) 1)))
  (if (`KismetArrayLibrary.Array_IsValidIndex` (`self.SessionsQuestionsPanel`) _output_get)
    (`self.AskQuestionEvent`)
    (else
      (`self.End Game`))))

(event `End Game`
  (`Widget.RemoveFromParent` (`self.AnswerWidget`))
  (bind _returnvalue (`|CreateWidget` "/Game/Quizz_UI/Quizz/WBP_EndGame.WBP_EndGame_C"))
  (set `self.EndWidget` _returnvalue)
  (`/Game/Quizz_UI/Quizz/WBP_EndGame.DisplayEndScreen` (`self.EndWidget`) (`self.TotalScore`) (`/Game/Quizz_Blueprints/GI_Quiz.TotalQuestions` (`self.BPGameInstance`)))
  (`KismetSystemLibrary.Delay` 15.0)
  (`GameplayStatics.OpenLevel` "MainMenu"))

(fn `BuildQuestionPanel`
  (returns (QuestionsReturned :type "Array of /Game/Quizz_Blueprints/ST_QuestionData Structure"))
  (locals (ReturnedQuestions :type "Array of /Game/Quizz_Blueprints/ST_QuestionData Structure"))
  (bind _bpgameinstance (`self.BPGameInstance`))
  (bind _outrownames (`DataTableFunctionLibrary.GetDataTableRowNames` "/Game/Quizz_Blueprints/DT_QuestionList.DT_QuestionList"))
  (set `self.AllQuestionsIDs` _outrownames)
  (if (`/Game/Quizz_Blueprints/GI_Quiz.RandomizeQuestions` _bpgameinstance)
    (`KismetArrayLibrary.Array_Shuffle` (`self.AllQuestionsIDs`)))
  (for _index (range (`/Game/Quizz_Blueprints/GI_Quiz.TotalQuestions` _bpgameinstance))
    ;[1 1 1] At each step of the loop : We take a random question name, add its data to the returned array of questions, and remove it from our panel at the end
    (bind _returnvalue (`|GetDataTableRow` "/Game/Quizz_Blueprints/DT_QuestionList.DT_QuestionList" (`|GetArrayItem` (`self.AllQuestionsIDs`) _index))
      (:`then`
        (`KismetArrayLibrary.Array_Add` (`local.ReturnedQuestions`) _returnvalue))))
  (return (`local.ReturnedQuestions`)))

(fn `CheckAnswer`
  (params (SelectedAnswer :type Text))
  (returns (IsAnswerGood :type Boolean))
  (bind _output (`self.GetCurrentQuestion`))
  (bind (_questiontext _answeroptions _correctanswers) (break `/Game/Quizz_Blueprints/ST_QuestionData` _output))
  (if (`KismetTextLibrary.EqualEqual_TextText` (`|GetArrayItem` _answeroptions (`|GetArrayItem` _correctanswers)) SelectedAnswer)
    (return true)
    (else
      (return false))))

(fn `GetCurrentQuestion`
  (returns (Output :type "/Game/Quizz_Blueprints/ST_QuestionData Structure"))
  ;[1 1 1] On récupère la question et les réponses de la question actuellement posée
  (return (`|GetArrayItem` (`self.SessionsQuestionsPanel`) (`self.CurrentQuestionIndex`))))

(fn `LoadNextQuestion`
  ;[1 1 1] Vérifie si nous sommes toujours dans les limites du nombre de questions, et si c'est le cas, passe à la question suivante
  (if (`KismetArrayLibrary.Array_IsValidIndex` (`self.SessionsQuestionsPanel`) (`self.CurrentQuestionIndex`))
    (bind _result (`/Engine/EditorBlueprintResources/StandardMacros.IncrementInt` (`self.CurrentQuestionIndex`))
      (:`  `
        (set `self.CurrentQuestionIndex` _result)))))

(fn `UserConstructionScript`
  (bind _asgi_quiz (cast `/Game/Quizz_Blueprints/GI_Quiz` (`GameplayStatics.GetGameInstance`)))
  (set `self.BPGameInstance` _asgi_quiz)
  (bind _questionsreturned (`self.BuildQuestionPanel`))
  (set `self.SessionsQuestionsPanel` _questionsreturned))